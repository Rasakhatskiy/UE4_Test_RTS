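; Test player controller that drives a top-down strategy-style camera through a TEST_CameraPawn reference cached on BeginPlay.
; Movement axes shift the pawn at a fixed height, while zoom actions change spring arm length within limits or reset it.
; Holding Pan rotates the pawn with clamped pitch and wraps the cursor across viewport edges.
; Otherwise, EdgeScroll turns cursor proximity to screen borders into local movement offsets.
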(event EventBeginPlay
  (Utilities|FlowControl|Sequence
    (:then_0
      (Utilities|ReferenceCast) ; Should be first
    )))

(event Input|ActionEvents|InputActionZoomReset
  (params (Key :type Key%20Structure :default "None"))
  ;[1 1 1] Zoom Control
  ;;[1 1 1] Reset Zoom
  (:Pressed
    (Variables|/Script/Engine.SpringArmComponent|SetTargetArmLength (Variables|/Game/Blueprints/TEST_CameraPawn.TEST_CameraPawn_C|GetSpringArm (Variables|References|GetCameraPawnRef)) (Variables|Zoom|GetDefaultZoomLength))))

(event Input|ActionEvents|InputActionZoomIn
  (params (Key :type Key%20Structure :default "None"))
  (bind _camerapawnref (Variables|References|GetCameraPawnRef))
  (bind _springarm (Variables|/Game/Blueprints/TEST_CameraPawn.TEST_CameraPawn_C|GetSpringArm _camerapawnref))
  ;[1 1 1] Zoom Control
  ;;[1 1 1] Zoom In
  (:Pressed
    (Variables|/Script/Engine.SpringArmComponent|SetTargetArmLength _springarm (Math|Float|Max(Float) (Variables|Zoom|GetMinZoomLimit) (- (Variables|/Script/Engine.SpringArmComponent|GetTargetArmLength _springarm) (Variables|Zoom|GetZoomSpeed))))))

(event Input|ActionEvents|InputActionZoomOut
  (params (Key :type Key%20Structure :default "None"))
  (bind _camerapawnref (Variables|References|GetCameraPawnRef))
  (bind _springarm (Variables|/Game/Blueprints/TEST_CameraPawn.TEST_CameraPawn_C|GetSpringArm _camerapawnref))
  ;[1 1 1] Zoom Control
  ;;[1 1 1] Zoom Out
  (:Pressed
    (Variables|/Script/Engine.SpringArmComponent|SetTargetArmLength _springarm (Math|Float|Min(Float) (+ (Variables|Zoom|GetZoomSpeed) (Variables|/Script/Engine.SpringArmComponent|GetTargetArmLength _springarm)) (Variables|Zoom|GetMaxZoomLimit)))))

(event Input|ActionEvents|InputActionPan
  (params (Key :type Key%20Structure :default "None"))
  ;[1 1 1] RMB Pressed
  (:Pressed
    (Variables|Rotate|SetIsPressed true))
  (:Released
    (Variables|Rotate|SetIsPressed false)))

(event Input|AxisEvents|InputAxisMoveForward
  (params (AxisValue :type Float%20%28single-precision%29))
  (bind _camerapawnref (Variables|References|GetCameraPawnRef))
  (bind _movementspeed (Variables|Movement|GetMovementSpeed))
  (bind _returnvalue (Transformation|GetActorTransform _camerapawnref))
  ;[1 1 1] Camera movement
  (Transformation|SetActorLocation _camerapawnref (Math|Vector|MakeVector (.X (Math|Vector|BreakVector (+ (Math|Transform|TransformDirection _returnvalue (Math|Vector|MakeVector (* AxisValue _movementspeed) (* _movementspeed (stale Input|AxisEvents|InputAxisMoveRight AxisValue)) 0.0)) (.Location (Math|Transform|BreakTransform _returnvalue))))) (.Y (Math|Vector|BreakVector (+ (Math|Transform|TransformDirection _returnvalue (Math|Vector|MakeVector (* AxisValue _movementspeed) (* _movementspeed (stale Input|AxisEvents|InputAxisMoveRight AxisValue)) 0.0)) (.Location (Math|Transform|BreakTransform _returnvalue))))) (Variables|Movement|GetDefaultActorHeight)) false false) ; Applying changes
)

(event Input|AxisEvents|InputAxisMoveRight
  (params (AxisValue :type Float%20%28single-precision%29))
  (bind _camerapawnref (Variables|References|GetCameraPawnRef))
  (bind _movementspeed (Variables|Movement|GetMovementSpeed))
  (bind _returnvalue (Transformation|GetActorTransform _camerapawnref))
  ;[1 1 1] Camera movement
  (Transformation|SetActorLocation _camerapawnref (Math|Vector|MakeVector (.X (Math|Vector|BreakVector (+ (Math|Transform|TransformDirection _returnvalue (Math|Vector|MakeVector (* (stale Input|AxisEvents|InputAxisMoveForward AxisValue) _movementspeed) (* _movementspeed AxisValue) 0.0)) (.Location (Math|Transform|BreakTransform _returnvalue))))) (.Y (Math|Vector|BreakVector (+ (Math|Transform|TransformDirection _returnvalue (Math|Vector|MakeVector (* (stale Input|AxisEvents|InputAxisMoveForward AxisValue) _movementspeed) (* _movementspeed AxisValue) 0.0)) (.Location (Math|Transform|BreakTransform _returnvalue))))) (Variables|Movement|GetDefaultActorHeight)) false false) ; Applying changes
)

(event Input|MouseEvents|Mouse2D
  (params (AxisValue :type Vector :default "0, 0, 0"))
  (bind (_x _y) (Math|Vector|BreakVector AxisValue))
  (bind (_locationx _locationy) (Game|Player|GetMousePosition))
  (bind (_sizex _sizey) (HUD|GetViewportSize))
  (bind _camerapawnref (Variables|References|GetCameraPawnRef))
  (bind _panspeed (Variables|Rotate|GetPanSpeed))
  (bind _defaultpitchangle (Variables|Rotate|GetDefaultPitchAngle))
  (bind _borderwidth (Variables|Rotate|GetBorderWidth))
  (bind _returnvalue (Transformation|GetActorRotation _camerapawnref))
  (bind _returnvalue_2 (Math|Float|Truncate _locationx))
  (bind _returnvalue_3 (Math|Float|Truncate _locationy))
  (bind _returnvalue_4 (- _sizey _borderwidth))
  (bind _returnvalue_5 (- _sizex _borderwidth))
  (Utilities|FlowControl|Sequence
    (:then_0
      ;[1 1 1] Pan Control
      (if (Variables|Rotate|GetIsPressed)
        (Transformation|SetActorRotation _camerapawnref (Math|Rotator|MakeRotator 0.0 (Math|Float|Clamp(Float) (+ (* _y _panspeed) (.pitch _returnvalue)) (- _defaultpitchangle 9e+01) _defaultpitchangle) (+ (* _x _panspeed) (.yaw _returnvalue))))
        ;[1 1 1] Mouse border teleporting
        (Utilities|FlowControl|Sequence
          (:then_0
            (if (< _returnvalue_2 _borderwidth)
              (Class|PlayerController|SetMouseLocation _returnvalue_5 _returnvalue_3) ; Move mouse to the right
            ))
          (:then_1
            (if (> _returnvalue_2 _returnvalue_5)
              (Class|PlayerController|SetMouseLocation _borderwidth _returnvalue_3) ; Move mouse to the left
            ))
          (:then_2
            (if (< _returnvalue_3 _borderwidth)
              (Class|PlayerController|SetMouseLocation _returnvalue_2 _returnvalue_4) ; Move mouse to the bottom
            ))
          (:then_3
            (if (> _returnvalue_3 _returnvalue_4)
              (Class|PlayerController|SetMouseLocation _returnvalue_2 _borderwidth) ; Move mouse to the top
            )))))
    (:then_1
      ;[1 1 1] Edge scroll
      (if (not (Variables|Rotate|GetIsPressed))
        (bind (_deltaspeedx _deltaspeedy) (Utilities|EdgeScroll))
        (Transformation|AddActorLocalOffset (Variables|References|GetCameraPawnRef) (Math|Vector|MakeVector _deltaspeedx _deltaspeedy 0.0) false false)))))

(fn ConstructionScript)